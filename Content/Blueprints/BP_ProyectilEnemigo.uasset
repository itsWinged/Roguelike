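; BP_ProyectilEnemigo is an enemy projectile that damages the player character on contact.
; The Collision component's overlap applies fixed damage only to player character 0, credits the instigator as damage causer, then destroys the projectile.
; It also destroys itself when ProjectileMovement stops or when the TiempoDespawn delay started at BeginPlay runs out.
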(event `self.ReceiveBeginPlay`
  (`KismetSystemLibrary.Delay` (`self.TiempoDespawn`))
  (`self.K2_DestroyActor`))

(event `self.Collision.OnComponentBeginOverlap`
  (params (OverlappedComponent :type "PrimitiveComponent Object Reference") (OtherActor :type "Actor Object Reference") (OtherComp :type "PrimitiveComponent Object Reference") (OtherBodyIndex :type Integer) (bFromSweep :type Boolean) (SweepResult :type "HitResult Structure (by ref)"))
  (if (== OtherActor (`GameplayStatics.GetPlayerCharacter` 0))
    (`GameplayStatics.ApplyDamage` OtherActor 1.0 null (`self.GetInstigator`))
    (`self.K2_DestroyActor`)))

(event `self.ProjectileMovement.OnProjectileStop`
  (params (ImpactResult :type "HitResult Structure (by ref)"))
  (`self.K2_DestroyActor`))

(fn `UserConstructionScript`)