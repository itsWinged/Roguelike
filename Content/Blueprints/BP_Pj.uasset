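; Player character with camera-relative movement, jumping, a chargeable bow and a spell-casting mode toggled by key 1.
; While casting, a per-tick camera trace moves a preview BP_SpellSpawn onto targeted LD_Casillas tiles, and left click spawns another there.
; Otherwise, holding left click charges arrow speed along a cubic ease-out, and release fires BP_Flecha and starts a cooldown.
; A gated Delay loop lets presses made during cooldown begin charging once it ends.
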(event `self.ReceiveBeginPlay`
  ;[1 1 1] Inicializacion
  (bind _outactors (`GameplayStatics.GetAllActorsOfClass` "/Game/Blueprints/BP_SpellSpawn.BP_SpellSpawn_C"))
  (set `self.SpellSpawn` (`KismetArrayLibrary.Array_Get` _outactors)))

(event `CastearHechizo`
  (if (`self.Casteando`)
    (`|SpawnActorFromClass` "/Game/Blueprints/BP_SpellSpawn.BP_SpellSpawn_C" (`KismetMathLibrary.MakeTransform` (`SceneComponent.K2_GetComponentLocation` (`.HitComponent` (`GameplayStatics.BreakHitResult` (stale `self.ReceiveTick` _outhit))))) "Undefined" "OverrideRootScale")
    (set `self.Casteando` false)))

(event `Key|One`
  (params (Key :type "Key Structure" :default "AnyKey"))
  ;[1 1 1] Casteo
  (:`Pressed`
    (if (`self.Casteando`)
      (set `self.Casteando` false)
      (set `self.puedeDisparar?` true)
      (else
        (set `self.Casteando` true)
        (set `self.puedeDisparar?` false)))))

(event `self.ReceiveTick`
  (params (DeltaSeconds :type "Float (single-precision)"))
  (bind _spellspawn (`self.SpellSpawn`))
  (bind _returnvalue (`SceneComponent.K2_GetComponentLocation` (`self.Camera`)))
  ;[1 1 1] Disparo arco
  (`|ExecutionSequence`
    (:`then_0`
      ;[1 1 1] Casteo
      (bind _outhit (`KismetSystemLibrary.LineTraceSingle` :`Start` _returnvalue :`End` (+ _returnvalue (* (`KismetMathLibrary.GetForwardVector` (`self.GetControlRotation`)) 5000)) :`TraceChannel` "TraceTypeQuery1" :`DrawTime` 5.0))
      (bind (_bblockinghit _binitialoverlap _time _location _impactpoint _normal _impactnormal _physmat _hitactor _hitcomponent) (`GameplayStatics.BreakHitResult` _outhit))
      (cast `/Game/LevelDesign/LD_Casillas` _hitactor ; Demasiado pesado?
        (:`then`
          (if (`self.Casteando`)
            (`self.K2_SetActorLocation` (`self.SpellSpawn`) (`SceneComponent.K2_GetComponentLocation` _hitcomponent) false false)
            (goto _label :!via `Reset`)
            (else
              _)))
        (:`CastFailed`
          _))
      (`/Engine/EditorBlueprintResources/StandardMacros.DoOnce` false :!label _label
        (:`Completed`
          (`self.K2_SetActorLocation` _spellspawn (`/Game/Blueprints/BP_SpellSpawn.PosicionReposo` _spellspawn) false false))))
    (:`then_1`
      (if (`self.puedeDisparar?`)
        (`/Engine/EditorBlueprintResources/StandardMacros.Gate` true :!label _label_2
          (:`Exit`
            (bind _output_get (set `self.contadorTiempo` (`KismetMathLibrary.FClamp` (+ DeltaSeconds (`self.contadorTiempo`)) 0.0 (`self.tiempoCargaArco`))))
            (bind _output_get_2 (set `self.velocidadFlecha` (- (`self.potenciaMaxArco`) (* (`KismetMathLibrary.MultiplyMultiply_FloatFloat` (- 0.0 (- (/ _output_get (`self.tiempoCargaArco`)) 1.0)) 3.0) (`self.potenciaMaxArco`)))))
            (`KismetSystemLibrary.PrintString` (`KismetStringLibrary.Concat_StrStr` "Potencia del arco: " (`KismetStringLibrary.Conv_DoubleToString` _output_get_2)) true true (struct :`G` 0.66 :`B` 1.0 :`A` 1.0) 0.001) ; feedback para testeo
          ))))))

(event `Key|LeftMouseButton`
  (params (Key :type "Key Structure" :default "AnyKey"))
  (bind _puededisparar_ (`self.puedeDisparar?`))
  ;[1 1 1] Disparo arco
  (:`Pressed`
    (`self.CastearHechizo`)
    ;;[1 1 1] Parafernalia para evitar bug con cooldown
    (`|ExecutionSequence`
      (:`then_0`
        (if _puededisparar_ :!label _label_3
          (goto _label_2 :!via `Open`)
          (else
            (`KismetSystemLibrary.Delay` 0.01)
            (`/Engine/EditorBlueprintResources/StandardMacros.Gate` false :!label _label_4
              (:`Exit`
                (if _puededisparar_
                  (goto _label_2 :!via `Open`)
                  (else
                    (goto _label_3))))))))
      (:`then_1`
        (goto _label_4 :!via `Open`))))
  (:`Released`
    (`|ExecutionSequence`
      (:`then_0`
        (if (`self.puedeDisparar?`)
          (`|ExecutionSequence`
            (:`then_0`
              (goto _label_2 :!via `Close`))
            (:`then_1`
              (bind _returnvalue (`|SpawnActorFromClass` "/Game/Blueprints/BP_Flecha.BP_Flecha_C" (`SceneComponent.K2_GetComponentToWorld` (`self.PuntoSpawnFlecha`)) "Undefined" "OverrideRootScale")) ; Primero spawneo y luego le doy la velocidad
              (`ProjectileMovementComponent.SetVelocityInLocalSpace` (`/Game/Blueprints/BP_Flecha.ProjectileMovement` _returnvalue) (`KismetMathLibrary.MakeVector` (`self.velocidadFlecha`))))
            (:`then_2`
              (set `self.velocidadFlecha` 0.0)
              (set `self.contadorTiempo` 0.0)
              (set `self.puedeDisparar?` false))
            (:`then_3`
              (`KismetSystemLibrary.Delay` (`self.cooldownDisparo`))
              (set `self.puedeDisparar?` true)))))
      (:`then_1`
        (goto _label_4 :!via `Close`)))))

(event `InputAxis|MoverAdelante`
  (params (AxisValue :type "Float (single-precision)"))
  ;[1 1 1] Movimiento
  (`self.AddMovementInput` (`KismetMathLibrary.GetForwardVector` (`KismetMathLibrary.MakeRotator` (.roll (`self.GetControlRotation`)) 0.0 (.yaw (`self.GetControlRotation`)))) AxisValue))

(event `InputAxis|MoverDerecha`
  (params (AxisValue :type "Float (single-precision)"))
  ;[1 1 1] Movimiento
  (`self.AddMovementInput` (`KismetMathLibrary.GetRightVector` (`KismetMathLibrary.MakeRotator` (.roll (`self.GetControlRotation`)) 0.0 (.yaw (`self.GetControlRotation`)))) AxisValue))

(event `InputAction|Saltar`
  (params (Key :type "Key Structure" :default "AnyKey"))
  (:`Pressed`
    (`self.Jump`)))

(event `InputAxis|Girar`
  (params (AxisValue :type "Float (single-precision)"))
  ;[1 1 1] Camara
  (`self.AddControllerYawInput` AxisValue))

(event `InputAxis|MirarArriba`
  (params (AxisValue :type "Float (single-precision)"))
  ;[1 1 1] Camara
  (`self.AddControllerPitchInput` AxisValue))

(fn `UserConstructionScript`)