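; LevelTest_sortida is a level exit trigger that streams in the next level when BP_Pj overlaps it.
; It finds the TargetPoint named NewLevelLocation and loads a level instance at its transform.
; The level is picked randomly from the InfoPersistente game instance's pool and removed to prevent repeats, with Boss_level used once the pool is empty.
; The marker and trigger destroy themselves so later loads find the correct ones.
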(event `CargaSiguienteNivel`
  (bind _outactors (`GameplayStatics.GetAllActorsOfClass` "/Script/Engine.TargetPoint" :!label _label)) ; busca el marcador de posicion del nuevo nivel
  (for _array_element _outactors
    (if (`KismetStringLibrary.EqualEqual_StrStr` (`KismetSystemLibrary.GetObjectName` _array_element) "NewLevelLocation")
      (bind _output_get (set `self.MarcadorPosicionNuevoNivel` _array_element))
      (set `self.TransformNuevoNivel` (`self.GetTransform` _output_get))
      (`|ExecutionSequence`
        (:`then_0`
          (break))
        (:`then_1`
          (bind _asinfo_persistente (cast `/Game/InfoPersistente` (`GameplayStatics.GetGameInstance`))) ; Accede a la info persistente
          (bind _poolniveles (`/Game/InfoPersistente.PoolNiveles` _asinfo_persistente))
          (set `self.PoolNivelesTemporal` _poolniveles)
          (if (== (`KismetArrayLibrary.Array_Length` (`self.PoolNivelesTemporal`)) 0)
            (set `self.NivelSeleccionado` "Boss_level")
            (else
              (set `self.NivelSeleccionado` (`KismetArrayLibrary.Array_Get` (`self.PoolNivelesTemporal`) (`KismetMathLibrary.RandomInteger` (`KismetArrayLibrary.Array_Length` _poolniveles))))))
          (`self.K2_DestroyActor` (`self.MarcadorPosicionNuevoNivel`)) ; destruye el marcador de posicion
          (`KismetArrayLibrary.Array_RemoveItem` _poolniveles (`self.NivelSeleccionado`)) ; Elimina el nivel de la pool para que no se repita
          (`LevelStreamingKismet.LoadLevelInstance` (`self.NivelSeleccionado`) (.location (`self.TransformNuevoNivel`)) (.rotation (`self.TransformNuevoNivel`))) ; carga el nivel en su posición y rotación
          (`self.K2_DestroyActor`) ; destruye el trigger para que no interfieran en la carga de los siguientes niveles
        )))))

(event `self.CollisionComponent.OnComponentBeginOverlap`
  (params (OverlappedComponent :type "PrimitiveComponent Object Reference") (OtherActor :type "Actor Object Reference") (OtherComp :type "PrimitiveComponent Object Reference") (OtherBodyIndex :type Integer) (bFromSweep :type Boolean) (SweepResult :type "HitResult Structure (by ref)"))
  (cast `/Game/Blueprints/BP_Pj` OtherActor) ; Cuando el pj entre en el trigger
  (goto _label))

(fn `UserConstructionScript`)