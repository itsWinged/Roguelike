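; Basic ranged enemy AI that chases the player (BP_Pj), firing cooldown-limited projectiles at their camera.
; Pawn sensing or player-dealt damage opens a never-closed gate, letting Tick run AIMoveTo, then turn and attack on arrival.
; Acceptance radius equals attack range while the player is seen, shrinking via retriggerable delay after sight is lost so the enemy closes in.
; Damage briefly swaps the mesh to a white material or destroys the actor at zero health.
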(event `self.ReceiveBeginPlay`
  ;[1 1 1] Inicialización
  (set `CharacterMovementComponent.MaxWalkSpeed` (`self.Velocidad`) (`self.CharacterMovement`))
  (set `self.MatInicial` (`PrimitiveComponent.GetMaterial` (`self.Mesh`) 0))
  (set `self.VidaActual` (`self.VidaMaxima`))
  (bind _outactors (`GameplayStatics.GetAllActorsOfClass` "/Game/Blueprints/BP_Pj.BP_Pj_C"))
  (set `self.PJ` (`KismetArrayLibrary.Array_Get` _outactors))
  (set `self.RangoAtkActual` (`self.RangoAtaque`)))

(event `self.ReceiveTick`
  (params (DeltaSeconds :type "Float (single-precision)"))
  (`/Engine/EditorBlueprintResources/StandardMacros.Gate` true :!label _label ; (temporalmente) cuando empieza a perseguir al jugador ya no para
    (:`Exit`
      (`|AIMoveTo` self (0.0 0.0 0.0) (`self.PJ`) (`self.RangoAtkActual`) ; movimiento IA basico
        (:`OnSuccess`
          (`self.K2_SetActorRotation` (`KismetMathLibrary.MakeRotator` 0.0 0.0 (.yaw (`KismetMathLibrary.FindLookAtRotation` (`self.K2_GetActorLocation`) (`self.K2_GetActorLocation` (`self.PJ`)))))) ; Cuando estés a rango míralo...
          (`self.Ataque`) ; ... y ataca
        )))))

(event `self.PawnSensing.OnSeePawn`
  (params (Pawn :type "Pawn Object Reference"))
  (`|ExecutionSequence`
    (:`then_0`
      (if (== Pawn (`self.PJ`))
        (set `self.RangoAtkActual` (`self.RangoAtaque`))
        (`self.PerseguirJugador`) ; persigue
      ))
    (:`then_1`
      (`KismetSystemLibrary.RetriggerableDelay` 0.6) ; Si no esta viendo al PJ quita el rango para que lo busque
      (set `self.RangoAtkActual` 5.0))))

(event `PerseguirJugador`
  (goto _label :!via `Open`))

(event `Ataque`
  (bind _posicionproyectil (`self.PosicionProyectil`))
  (if (`self.PuedeAtacar`)
    (`|SpawnActorFromClass` "/Game/Blueprints/BP_ProyectilEnemigo.BP_ProyectilEnemigo_C" (`KismetMathLibrary.MakeTransform` (`SceneComponent.K2_GetComponentLocation` _posicionproyectil) (`KismetMathLibrary.FindLookAtRotation` (`SceneComponent.K2_GetComponentLocation` _posicionproyectil) (`SceneComponent.K2_GetComponentLocation` (`/Game/Blueprints/BP_Pj.Camera` (`self.PJ`))))) "Undefined" "OverrideRootScale" null self)
    ;[1 1 1] cooldown ataque
    (set `self.PuedeAtacar` false)
    (`KismetSystemLibrary.Delay` (`self.CooldownAtaque`))
    (set `self.PuedeAtacar` true)))

(event `self.ReceiveAnyDamage`
  (params (Damage :type "Float (single-precision)") (DamageType :type "DamageType Object Reference") (InstigatedBy :type "Controller Object Reference") (DamageCauser :type "Actor Object Reference"))
  (`|ExecutionSequence`
    (:`then_0`
      (set `self.VidaActual` (- (`self.VidaActual`) Damage))
      (if (<= (`self.VidaActual`) 0.0)
        (`self.K2_DestroyActor`)
        (else
          (`PrimitiveComponent.SetMaterial` (`self.Mesh`) 0 (`self.MatBlanco`))
          (`KismetSystemLibrary.RetriggerableDelay` 0.5)
          (`PrimitiveComponent.SetMaterial` (`self.Mesh`) 0 (`self.MatInicial`)))))
    (:`then_1`
      (if (== DamageCauser (`self.PJ`))
        (`self.PerseguirJugador`)))))

(fn `UserConstructionScript`)