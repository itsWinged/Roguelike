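; Basic melee enemy AI that chases the player (BP_Pj) and damages them at close range.
; Seeing the player or taking damage from them opens a gate that lets Tick issue AIMoveTo every frame, with nothing closing it afterward.
; An attack-range overlap starts a self-repeating, cooldown-limited attack while the player stays inside.
; Damage reduces health, briefly flashes a white material via retriggerable delay, and destroys the actor at zero.
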(event `self.ReceiveBeginPlay`
  (set `CharacterMovementComponent.MaxWalkSpeed` (`self.Velocidad`) (`self.CharacterMovement`))
  (set `self.MatInicial` (`PrimitiveComponent.GetMaterial` (`self.Mesh`) 0))
  (set `self.VidaActual` (`self.VidaMaxima`))
  (bind _outactors (`GameplayStatics.GetAllActorsOfClass` "/Game/Blueprints/BP_Pj.BP_Pj_C"))
  (set `self.PJ` (`KismetArrayLibrary.Array_Get` _outactors)))

(event `self.ReceiveTick`
  (params (DeltaSeconds :type "Float (single-precision)"))
  (`/Engine/EditorBlueprintResources/StandardMacros.Gate` true :!label _label
    (:`Exit`
      (`|AIMoveTo` self (0.0 0.0 0.0) (`self.PJ`) 100.0))))

(event `self.PawnSensing.OnSeePawn`
  (params (Pawn :type "Pawn Object Reference"))
  (if (== Pawn (`self.PJ`))
    (`self.PerseguirJugador`)))

(event `PerseguirJugador`
  (goto _label :!via `Open`))

(event `self.RangoAtaque.OnComponentBeginOverlap`
  (params (OverlappedComponent :type "PrimitiveComponent Object Reference") (OtherActor :type "Actor Object Reference") (OtherComp :type "PrimitiveComponent Object Reference") (OtherBodyIndex :type Integer) (bFromSweep :type Boolean) (SweepResult :type "HitResult Structure (by ref)"))
  (bind _asbp_pj (cast `/Game/Blueprints/BP_Pj` OtherActor))
  (set `self.PjADanyar` _asbp_pj)
  (set `self.EstaARango` true)
  (`self.Ataque`))

(event `self.RangoAtaque.OnComponentEndOverlap`
  (params (OverlappedComponent :type "PrimitiveComponent Object Reference") (OtherActor :type "Actor Object Reference") (OtherComp :type "PrimitiveComponent Object Reference") (OtherBodyIndex :type Integer))
  (cast `/Game/Blueprints/BP_Pj` OtherActor)
  (set `self.EstaARango` false))

(event `Ataque`
  (if (and (`self.EstaARango`) (`self.PuedeAtacar`))
    (`GameplayStatics.ApplyDamage` (`self.PjADanyar`) (`self.DanyoAtaque`))
    (set `self.PuedeAtacar` false)
    (`KismetSystemLibrary.Delay` (`self.CooldownAtaque`))
    (set `self.PuedeAtacar` true)
    (`self.Ataque`)))

(event `self.ReceiveAnyDamage`
  (params (Damage :type "Float (single-precision)") (DamageType :type "DamageType Object Reference") (InstigatedBy :type "Controller Object Reference") (DamageCauser :type "Actor Object Reference"))
  (`|ExecutionSequence`
    (:`then_0`
      (set `self.VidaActual` (- (`self.VidaActual`) Damage))
      (if (<= (`self.VidaActual`) 0.0)
        (`self.K2_DestroyActor`)
        (else
          (`PrimitiveComponent.SetMaterial` (`self.Mesh`) 0 (`self.MatBlanco`))
          (`KismetSystemLibrary.RetriggerableDelay` 0.5)
          (`PrimitiveComponent.SetMaterial` (`self.Mesh`) 0 (`self.MatInicial`)))))
    (:`then_1`
      (if (== DamageCauser (`self.PJ`))
        (`self.PerseguirJugador`)))))

(fn `UserConstructionScript`)