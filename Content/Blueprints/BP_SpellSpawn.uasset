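; BP_SpellSpawn shows a preview for the player's currently selected spell.
; On BeginPlay it finds the BP_Pj character and maps spell enum values to preview components (spike-spitting totem, ground burn, acid flask), with the other mapped spells sharing an empty "Ninguno" one.
; CambioHechizo hides every preview, then reveals the one mapped to HechizoSeleccionado.
; An unconnected leftover would spawn the selected spell's class at PosicionReposo.
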(event `CambioHechizo`
  ;[1 1 1] Cuando se cambie de hechizo enseña solo esa prev
  (for _array_element (`self.Prevs`)
    (`SceneComponent.SetVisibility` _array_element false true))
  (`SceneComponent.SetVisibility` (`BlueprintMapLibrary.Map_Find` (`self.HechizoParaPrev`) (`/Game/Blueprints/BP_Pj.HechizoSeleccionado` (`self.PJ`))) true true))

(event `self.ReceiveBeginPlay`
  (bind _ninguno (`self.ninguno`))
  (bind _hechizoparaprev (`self.HechizoParaPrev`))
  (bind _outactors (`GameplayStatics.GetAllActorsOfClass` "/Game/Blueprints/BP_Pj.BP_Pj_C"))
  (set `self.PJ` (`KismetArrayLibrary.Array_Get` _outactors))
  (set `self.Prevs` (`|MakeArray` (`self.TotemEscupepinchos`) (`self.QuemarSuelo`) (`self.FrascoAcido`) (`self.ninguno`))) ; Crea un array con todas las prevs para poder esconderlas después
  (`BlueprintMapLibrary.Map_Add` _hechizoparaprev "NewEnumerator5" (`self.TotemEscupepinchos`))
  (`BlueprintMapLibrary.Map_Add` _hechizoparaprev "NewEnumerator8" (`self.QuemarSuelo`))
  (`BlueprintMapLibrary.Map_Add` _hechizoparaprev "NewEnumerator3" (`self.FrascoAcido`))
  (`BlueprintMapLibrary.Map_Add` _hechizoparaprev "NewEnumerator0" _ninguno)
  (`BlueprintMapLibrary.Map_Add` _hechizoparaprev "NewEnumerator1" _ninguno)
  (`BlueprintMapLibrary.Map_Add` _hechizoparaprev "NewEnumerator4" _ninguno)
  (`BlueprintMapLibrary.Map_Add` _hechizoparaprev "NewEnumerator6" _ninguno)
  (`BlueprintMapLibrary.Map_Add` _hechizoparaprev "NewEnumerator7" _ninguno)
  (`BlueprintMapLibrary.Map_Add` _hechizoparaprev "NewEnumerator9" _ninguno)
  (`self.CambioHechizo`))

(event `Key|Y`
  (params (Key :type "Key Structure" :default "AnyKey")))

(fn `UserConstructionScript`)